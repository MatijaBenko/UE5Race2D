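; BP_MyGameModeBase is a game mode Blueprint that owns the timer HUD and its win and lose messages.
; On BeginPlay it creates the WB_Timer widget, adds it to the viewport, sets a starting time and hides both result texts.
; It binds handlers to time-changed, lost and win delegates, which forward the new time or visibility to the widget.
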(event Custom|OnTimeChangedDelegateFired
  (params (NewTimer :type Float%20%28single-precision%29))
  (Default|SetTimerText (Variables|Default|GetTimerHub) NewTimer))

(event Custom|OnLostDelegateFired
  (params (IsVisible :type ESlateVisibility%20Enum :default "Visible"))
  (Default|SetLostText (Variables|Default|GetTimerHub) IsVisible))

(event Custom|OnWinDelegatedFired
  (params (IsVisible :type ESlateVisibility%20Enum :default "Visible"))
  (Default|SetWinText (Variables|Default|GetTimerHub) IsVisible))

(event EventBeginPlay
  (bind _returnvalue (UserInterface|CreateWidget "/Game/Blueprints/UserWidgets/WB_Timer.WB_Timer_C"))
  (Variables|Default|SetTimerHub _returnvalue)
  (Widget|SetVisibility (Variables|Default|GetTimerHub) "Visible")
  (UserInterface|Viewport|AddtoViewport (Variables|Default|GetTimerHub) 0)
  (Default|SetTimerText (Variables|Default|GetTimerHub) 1e+02)
  (EventDispatchers|BindEventtoTimeChangedDelegate (delegate Custom|OnTimeChangedDelegateFired))
  (Default|SetLostText (Variables|Default|GetTimerHub) "Hidden")
  (EventDispatchers|BindEventtoLostTextDelegate (delegate Custom|OnLostDelegateFired))
  (Default|SetWinText (Variables|Default|GetTimerHub) "Hidden")
  (EventDispatchers|BindEventtoWinTextDelegate (delegate Custom|OnWinDelegatedFired)))

(event EventTick
  (params (DeltaSeconds :type Float%20%28single-precision%29)))

(fn ConstructionScript)